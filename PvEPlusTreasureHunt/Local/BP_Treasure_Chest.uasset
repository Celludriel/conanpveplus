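; Locked treasure chest for a Conan Exiles treasure hunt, opened only with a key carrying its matching TreasureChestId.
; Clearing its linked SpawnCache drops that key in a loot bag and starts a short despawn timer on the chest.
; First opening consumes the key, fills loot from a data table row and notifies other characters who know of the treasure.
; An unclaimed chest self-destructs after a long server-side timeout, notifying those characters.
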(event `InteractableInterface.InteractableActivate`
  (params (Component :type "PrimitiveComponent Object Reference") (Instigator :type "PlayerController Object Reference") (HitIndex :type Integer))
  (bind _returnvalue (`self.GetComponentByClass` "/Game/Systems/Loot/TableSetup/BP_AC_LootSpawner.BP_AC_LootSpawner_C"))
  (bind _asconan_character (cast `ConanCharacter` (`Controller.K2_GetPawn` Instigator) :!pure true))
  (if (`self.HasBeenOpened`)
    (`parent.InteractableActivate` Component Instigator HitIndex)
    (else
      (bind _returnvalue_2 (`ConanCharacter.GetBackpackInventory` _asconan_character))
      (bind _keyindex (`self.CheckIfInventoryContainsKeyWithTreasureChestId` _returnvalue_2)
        (:`Completed`
          (if (`self.HasKey`)
            (set `/Game/Systems/Loot/TableSetup/BP_AC_LootSpawner.LootHasBeenSpawned` true _returnvalue)
            (set `/Game/Systems/Loot/TableSetup/BP_AC_LootSpawner.ReplenishLoot?` false _returnvalue)
            (`parent.InteractableActivate` Component Instigator HitIndex)
            (`ItemInventory.DeleteItems` _returnvalue_2 _keyindex 1)
            (if (not (`self.HasBeenOpened`))
              (`self.NotifyPlayersOfOpenedChest` _asconan_character
                (:`Out`
                  (set `self.HasBeenOpened` true)
                  (`self.SpawnLootAfterOpening`))))
            (else
              (`ConanCharacter.ClientHUDShowNotification` _asconan_character (`self.MustHaveKey`) false))))))))

(event `self.ReceiveBeginPlay`
  (if (`KismetSystemLibrary.IsServer`)
    (`KismetSystemLibrary.Delay` 5.0)
    (`KismetSystemLibrary.K2_SetTimerDelegate` (delegate `DestroyChestAfterTimeout`) 43200.0)
    (add `/Game/Mods/PvEPlusTreasureHunt/SpawnCache.CacheHasBeenCleared` (`self.SpawnCache`) (delegate `SpawnKey`))))

(event `SpawnKey`
  (params (Location :type "Vector Structure"))
  (`self.SpawnKeyAfterBossDeath` Location)
  (set `self.MarkedForDespawn` true)
  (`KismetSystemLibrary.K2_SetTimerDelegate` (delegate `DespawnChest`) 120.0))

(event `DestroyChestAfterTimeout`
  (if (not (`self.MarkedForDespawn`))
    (`self.DestroyChestActorAfterTimeout`)))

(event `DespawnChest`
  (`self.K2_DestroyActor`))

(fn `AddConanCharacterThatKnowsOfTreasure`
  (params (`Conan Character` :type "ConanCharacter Object Reference"))
  (`KismetArrayLibrary.Array_Add` (`self.ConanCharactersThatKnowsOfTreasure`) `Conan Character`))

(fn `UserConstructionScript`
  (`parent.UserConstructionScript`))