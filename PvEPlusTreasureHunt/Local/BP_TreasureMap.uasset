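; Treasure map item that, when used, opens a map UI showing the treasure locations known to the using character.
; Outside the server, it activates the TreasureMap GUI module if inactive and reads locations from the character's BP_Treasure_Location_Placeholder component.
; World X/Y are shifted by hard-coded offsets, scaled to image size, and used as overlay padding to place tinted stamp markers.
; It then centers both map scroll boxes.
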(event `self.OnUseItem`
  (params (invokingCharacter :type "ConanCharacter Object Reference"))
  (bind _returnvalue (`GUIModuleController.GetGUIModuleController`))
  (if (`KismetSystemLibrary.IsServer`)
    _
    (elif (not (`GUIModuleController.IsModuleActive` _returnvalue "TreasureMap"))
      (bind _returnvalue_2 (`GUIModuleController.ActivateModule` _returnvalue "TreasureMap" true false))
      (for _array_element (`/Game/Mods/PvEPlusTreasureHunt/BP_Treasure_Location_Placeholder.KnownTreasureLocations` (`Actor.GetComponentByClass` invokingCharacter "/Game/Mods/PvEPlusTreasureHunt/BP_Treasure_Location_Placeholder.BP_Treasure_Location_Placeholder_C"))
        (bind _asw_treasure_map (cast `/Game/Mods/PvEPlusTreasureHunt/W_TreasureMap` _returnvalue_2 :!pure true))
        (`self.ShowMarkerOnMap` _array_element _asw_treasure_map))
      (`self.CenterMap` _asw_treasure_map))))

(fn `CanUseItem`
  (params (invokingCharacter :type "ConanCharacter Object Reference"))
  (returns (ReturnValue :type Boolean))
  (return true))

(fn `CartesianToMapGrid`
  (params (WorldLocation :type "Vector Structure"))
  (returns (MapGridX :type "Float (double-precision)") (MapGridY :type "Float (double-precision)"))
  (bind _returnvalue (/ (`self.WorldDimension`) 2.0))
  (return (+ _returnvalue (- (.x WorldLocation) 65000.0)) (+ _returnvalue (+ (.y WorldLocation) 35000.0))))

(fn `CartesianWorldToMapCoordinates`
  (params (WorldLocation :type "Vector Structure"))
  (returns (MapX :type "Float (double-precision)") (MapY :type "Float (double-precision)"))
  (bind (_mapgridx _mapgridy) (`self.CartesianToMapGrid` WorldLocation))
  (bind _mapcoordinate (`self.WorldDimensionToMapImageDimension` _mapgridx))
  (bind _mapcoordinate_2 (`self.WorldDimensionToMapImageDimension` _mapgridy))
  (return _mapcoordinate _mapcoordinate_2))

(fn `CenterMap`
  (params (WTreasureMap :type "/Game/Mods/PvEPlusTreasureHunt/W_TreasureMap Object Reference"))
  (`self.MoveScrollBarToCenter` (`/Game/Mods/PvEPlusTreasureHunt/W_TreasureMap.HScrollBox` WTreasureMap))
  (`self.MoveScrollBarToCenter` (`/Game/Mods/PvEPlusTreasureHunt/W_TreasureMap.VScrollBox` WTreasureMap)))

(fn `MoveScrollBarToCenter`
  (params (ScrollBar :type "ScrollBox Object Reference"))
  (`ScrollBox.ScrollWidget` ScrollBar (/ (`ScrollBox.GetMaxScrollOffset` ScrollBar) 2.0))
  (`Widget.ForceLayoutPrepass` ScrollBar))

(fn `ShowMarkerOnMap`
  (params (TreasureLocation :type "Vector Structure") (WTreasureMap :type "/Game/Mods/PvEPlusTreasureHunt/W_TreasureMap Object Reference"))
  (bind (_mapx _mapy) (`self.CartesianWorldToMapCoordinates` TreasureLocation))
  (bind _returnvalue (`|CreateWidget` "/Game/UI/Map/w_MapMarkerView.W_MapMarkerView_C"))
  (bind _markerimage (`/Game/UI/Map/w_MapMarkerView.MarkerImage` _returnvalue))
  (`Image.SetBrushFromTexture` _markerimage "/Game/UI/Textures/GUIs/Map/T_Map_Icon_stamp_treasure.T_Map_Icon_stamp_treasure" false)
  (`Image.SetColorAndOpacity` _markerimage (struct :`R` 1.0 :`G` 0.517744 :`B` 0.038727 :`A` 1.0))
  (bind _returnvalue_2 (`PanelWidget.AddChild` (`/Game/Mods/PvEPlusTreasureHunt/W_TreasureMap.MarkerOverlay` WTreasureMap) _returnvalue))
  (`OverlaySlot.SetPadding` (cast `OverlaySlot` _returnvalue_2 :!pure true) (make `Margin` _mapx _mapy)))

(fn `WorldDimensionToMapImageDimension`
  (params (WorldCoordinate :type "Float (double-precision)"))
  (returns (MapCoordinate :type "Float (double-precision)"))
  (return (* WorldCoordinate (/ (`self.MapImageDimension`) (`self.WorldDimension`)))))