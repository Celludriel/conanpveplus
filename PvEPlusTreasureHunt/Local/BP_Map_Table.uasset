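; BP_Map_Table is an interactable map table that opens the TreasureMap GUI module on the client and marks every BP_Treasure_Chest on it.
; Each chest's world location is shifted by hardcoded offsets and half the world dimension, then scaled to map image size.
; A tinted stamp marker widget is added to the map's overlay, positioned through slot padding.
; Each marker's coordinates are also printed on screen as debug text.
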(event `InteractableInterface.ClientInteractableActivate`
  (params (Component :type "PrimitiveComponent Object Reference") (Instigator :type "PlayerController Object Reference") (HitIndex :type Integer))
  (bind _returnvalue (`GUIModuleController.ActivateModule` (`GUIModuleController.GetGUIModuleController`) "TreasureMap" true false))
  (bind _outactors (`GameplayStatics.GetAllActorsOfClass` "/Game/Mods/PvEPlusTreasureHunt/BP_Treasure_Chest.BP_Treasure_Chest_C"))
  (for _array_element _outactors
    (bind (_mapx _mapy) (`self.CartesianWorldToMapCoordinates` (`self.K2_GetActorLocation` _array_element)))
    (bind _returnvalue_2 (`|CreateWidget` "/Game/UI/Map/w_MapMarkerView.W_MapMarkerView_C"))
    (bind _markerimage (`/Game/UI/Map/w_MapMarkerView.MarkerImage` _returnvalue_2))
    (`Image.SetBrushFromTexture` _markerimage "/Game/UI/Textures/GUIs/Map/T_Map_Icon_stamp_treasure.T_Map_Icon_stamp_treasure" false)
    (`Image.SetColorAndOpacity` _markerimage (struct :`R` 1.0 :`G` 0.517744 :`B` 0.038727 :`A` 1.0))
    (bind _returnvalue_3 (`PanelWidget.AddChild` (`/Game/Mods/PvEPlusTreasureHunt/W_TreasureMap.MarkerOverlay` (cast `/Game/Mods/PvEPlusTreasureHunt/W_TreasureMap` _returnvalue :!pure true)) _returnvalue_2))
    (`OverlaySlot.SetPadding` (cast `OverlaySlot` _returnvalue_3 :!pure true) (make `Margin` _mapx _mapy))
    (`KismetSystemLibrary.PrintString` (`KismetStringLibrary.BuildString_Double` (`KismetStringLibrary.BuildString_Double` "" "WorldMapCoord x [" _mapx "] ") "y [" _mapy "]") true true (struct :`G` 0.66 :`B` 1.0 :`A` 1.0) 30.0)))

(fn `CartesianToMapGrid`
  (params (WorldLocation :type "Vector Structure"))
  (returns (MapGridX :type "Float (double-precision)") (MapGridY :type "Float (double-precision)"))
  (bind _returnvalue (/ (`self.WorldDimension`) 2.0))
  (return (+ _returnvalue (- (.x WorldLocation) 65000.0)) (+ _returnvalue (+ (.y WorldLocation) 35000.0))))

(fn `CartesianWorldToMapCoordinates`
  (params (WorldLocation :type "Vector Structure"))
  (returns (MapX :type "Float (double-precision)") (MapY :type "Float (double-precision)"))
  (bind (_mapgridx _mapgridy) (`self.CartesianToMapGrid` WorldLocation))
  (bind _mapcoordinate (`self.WorldDimensionToMapImageDimension` _mapgridx))
  (bind _mapcoordinate_2 (`self.WorldDimensionToMapImageDimension` _mapgridy))
  (return _mapcoordinate _mapcoordinate_2))

(fn `UserConstructionScript`
  (`parent.UserConstructionScript`))

(fn `WorldDimensionToMapImageDimension`
  (params (WorldCoordinate :type "Float (double-precision)"))
  (returns (MapCoordinate :type "Float (double-precision)"))
  (return (* WorldCoordinate (/ (`self.MapImageDimension`) (`self.WorldDimension`)))))