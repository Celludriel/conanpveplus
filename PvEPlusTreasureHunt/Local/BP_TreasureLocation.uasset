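; Usable treasure map item that, on the server, reveals a treasure location suited to the player's level.
; Shuffles eligible TreasureMapTable rows, skipping spots near player foundations or a chest marked for despawn.
; An empty spot spawns BP_Treasure_Chest with loot ID, boss spawn and the user registered as knowing it; an existing chest is only announced.
; Either reveal consumes the map; finding no spot reports a fake map and keeps it.
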(event `self.OnUseItem`
  (params (invokingCharacter :type "ConanCharacter Object Reference"))
  (if (`KismetSystemLibrary.IsServer`)
    (bind _asconan_player_controller (cast `ConanPlayerController` (`/Game/Characters/FuncomFunctionLibrary.GetControllerFromActor` invokingCharacter))
      (:`then`
        (bind (_treasuremapdata _found _alreadyspawned) (`self.FindTreasureLocation` invokingCharacter))
        (if _found
          (if (not _alreadyspawned)
            (`self.NewTreasureRevealed` (break `/Game/Mods/PvEPlusTreasureHunt/TreasureMapData` _treasuremapdata) (`.BossProtector_8_B2AAB5EC45D0E26BBAD46FA8AAE76ADD` (break `/Game/Mods/PvEPlusTreasureHunt/TreasureMapData` _treasuremapdata)) (`.TreasureLootId_16_8532979B4D9F676C2430BBB3F2A60A34` (break `/Game/Mods/PvEPlusTreasureHunt/TreasureMapData` _treasuremapdata)) invokingCharacter)
            (else
              (`self.ExistingTreasureRevealed` _asconan_player_controller)))
          (else
            (`ConanPlayerController.ClientHUDShowNotification` _asconan_player_controller (`KismetTextLibrary.Conv_StringToText` "It appears this map was a fake no treasure has been revealed") true))))
      (:`CastFailed`
        (`LoggerLibrary.DWLogString` "Cast To ConanPlayerController Failed" "Modding" "INFOL_CODEERROR")))))

(fn `CanUseItem`
  (params (invokingCharacter :type "ConanCharacter Object Reference"))
  (returns (ReturnValue :type Boolean))
  (return true))

(fn `DeleteItem`
  (params (Item :type "GameItem Object Reference"))
  (bind _returnvalue (`self.GetOwnerInventory` Item))
  (`ItemInventory.DeleteItems` _returnvalue (`ItemInventory.GetItemIndex` _returnvalue Item) 1))

(fn `FindTreasureLocation`
  (params (ConanCharacter :type "ConanCharacter Object Reference"))
  (returns (TreasureMapData :type "/Game/Mods/PvEPlusTreasureHunt/TreasureMapData Structure") (found :type Boolean) (AlreadySpawned :type Boolean))
  (locals (AvailableTreasureLocationsForLevel :type "Array of /Game/Mods/PvEPlusTreasureHunt/TreasureMapData Structure"))
  (bind _availabletreasurelocationsforlevel (`local.AvailableTreasureLocationsForLevel`))
  (bind _item (`KismetArrayLibrary.Array_Get` _availabletreasurelocationsforlevel))
  (bind _location (break `/Game/Mods/PvEPlusTreasureHunt/TreasureMapData` _item))
  (`KismetArrayLibrary.Array_Clear` (`local.AvailableTreasureLocationsForLevel`))
  (bind _outrownames (`DataTableFunctionLibrary.GetDataTableRowNames` "/Game/Mods/PvEPlusTreasureHunt/TreasureMapTable.TreasureMapTable"))
  (for _array_element _outrownames
    (bind _returnvalue (`|GetDataTableRow` "/Game/Mods/PvEPlusTreasureHunt/TreasureMapTable.TreasureMapTable" _array_element)
      (:`then`
        (if (<= (`.MinimumLevel_5_491FB291451CDE2A7F8A1AB7C6BD4A25` (break `/Game/Mods/PvEPlusTreasureHunt/TreasureMapData` _returnvalue)) (`ConanCharacter.GetIntStat` ConanCharacter "Level" "Full"))
          (`KismetArrayLibrary.Array_Add` _availabletreasurelocationsforlevel _returnvalue)))))
  (if (> (`KismetArrayLibrary.Array_Length` _availabletreasurelocationsforlevel) 0) :!label _label
    (`KismetArrayLibrary.Array_Shuffle` _availabletreasurelocationsforlevel)
    (bind (_outactors _returnvalue_2) (`KismetSystemLibrary.SphereOverlapActors` _location 5000.0 (`|MakeArray` "ObjectTypeQuery10" :!type "EObjectTypeQuery Enum") "/Game/Systems/Building/BP_BuildFoundation.BP_BuildFoundation_C"))
    (if (not _returnvalue_2)
      (bind _chestispresent (`self.CheckForTreasureChest` _location)
        (:`FindAnotherSpot`
          _)
        (:`SpotCanBeUsed`
          (return _item true _chestispresent))))
    (`KismetArrayLibrary.Array_RemoveItem` (`local.AvailableTreasureLocationsForLevel`) _item)
    (goto _label)
    (else
      (return (struct) false false))))