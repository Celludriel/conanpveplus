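; Function library that spawns and configures NPCs, either directly from a class or by finishing an async spawn-table spawn.
; Both paths snap the NPC to the closest walkable hit of a vertical capsule trace, destroying it if none exists.
; Configuration sets spawner data and behavior parameters, randomizing human looks and weapons from data tables for non-table spawns.
; Table spawns instead apply the supplied layout and refill health, stamina and consciousness.
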(fn `CheckForInvalidDataTableValues`
  (params (DataTableRow :type "/Game/Systems/Spawning/Humans/NPC_Human_Visuals_Structure Structure (by ref)"))
  (returns (VisPieces :type "Array of Integer"))
  (locals (TempNPCCreationArray :type "Array of Integer"))
  (bind (_var1 _var2 _var3 _var4 _var5 _var6 _var7 _var8 _var9 _var10 _var11 _var12 _var13 _var14 _var15) (break `/Game/Systems/Spawning/Humans/NPC_Human_Visuals_Structure` DataTableRow))
  (bind _tempnpccreationarray (`local.TempNPCCreationArray`))
  (`KismetArrayLibrary.Array_Clear` (`local.TempNPCCreationArray`))
  (if (> _var1 -1)
    (`KismetArrayLibrary.Array_Add` _tempnpccreationarray _var1)
    (if (> _var2 -1)
      (`KismetArrayLibrary.Array_Add` _tempnpccreationarray _var2)
      (if (> _var3 -1)
        (`KismetArrayLibrary.Array_Add` _tempnpccreationarray _var3)
        (if (> _var4 -1)
          (`KismetArrayLibrary.Array_Add` _tempnpccreationarray _var4)
          (if (> _var5 -1)
            (`KismetArrayLibrary.Array_Add` _tempnpccreationarray _var5)
            (if (> _var6 -1)
              (`KismetArrayLibrary.Array_Add` _tempnpccreationarray _var6)
              (if (> _var7 -1)
                (`KismetArrayLibrary.Array_Add` _tempnpccreationarray _var7)
                (if (> _var8 -1)
                  (`KismetArrayLibrary.Array_Add` _tempnpccreationarray _var8)
                  (if (> _var9 -1)
                    (`KismetArrayLibrary.Array_Add` _tempnpccreationarray _var9)
                    (if (> _var10 -1)
                      (`KismetArrayLibrary.Array_Add` _tempnpccreationarray _var10)
                      (if (> _var11 -1)
                        (`KismetArrayLibrary.Array_Add` _tempnpccreationarray _var11)
                        (if (> _var12 -1)
                          (`KismetArrayLibrary.Array_Add` _tempnpccreationarray _var12)
                          (if (> _var13 -1)
                            (`KismetArrayLibrary.Array_Add` _tempnpccreationarray _var13)
                            (if (> _var14 -1)
                              (`KismetArrayLibrary.Array_Add` _tempnpccreationarray _var14)
                              (if (> _var15 -1)
                                (`KismetArrayLibrary.Array_Add` _tempnpccreationarray _var15))))))))))))))))
  (return (`local.TempNPCCreationArray`)))

(fn `ConfigureSpawnedNPC`
  (params (HumanNPCType :type "/Game/Systems/Spawning/SpawnInputs/NPCHumans Enum") (`Human?` :type Boolean) (NPC :type "/Game/Characters/BaseNPC Object Reference") (SpawnerHumanNPCIndex :type Integer) (SpawnerWIldlifeNPCIndex :type Integer) (SpawnerStaticSpawnpointIndex :type Integer) (RoamRadius :type "Float (double-precision)") (SpawnLocation :type "Vector Structure") (StaticSpawnPoint :type "StaticSpawnPoint Object Reference") (`Territory Volume Spawner` :type "/Game/Systems/AI/BP_NPCTerritorySpawnerInterface Interface") (BehaviorParameters :type "/Game/Systems/AI/BP_NPCBehaviorParameters Object Reference") (SpawnedFromSpawnTable :type Boolean) (Name :type Text) (RowName :type Name))
  (locals (bSpawnedFromSpawnTable :type Boolean))
  (if (== (`ConanCharacter.SourceSpawnTable` NPC) "None")
    (`ConanCharacter.SetCharacterSpawnTableID` NPC RowName))
  (set `local.bSpawnedFromSpawnTable` SpawnedFromSpawnTable)
  (set `/Game/Characters/BaseNPC.Territory Volume Spawner` `Territory Volume Spawner` NPC)
  (set `/Game/Characters/BaseNPC.SpawnPoint` StaticSpawnPoint NPC)
  (if (`KismetSystemLibrary.IsValid` StaticSpawnPoint)
    (set `/Game/Characters/BaseNPC.SpawnerType` "ManualSpawner" NPC)
    (set `/Game/Characters/BaseNPC.NPC Territory Group` SpawnerStaticSpawnpointIndex NPC)
    (elif `Human?`
      (set `/Game/Characters/BaseNPC.SpawnerType` "HumanNPC" NPC)
      (set `/Game/Characters/BaseNPC.NPC Territory Group` SpawnerHumanNPCIndex NPC)
      (else
        (set `/Game/Characters/BaseNPC.SpawnerType` "WildlifeNPC" NPC)
        (set `/Game/Characters/BaseNPC.NPC Territory Group` SpawnerWIldlifeNPCIndex NPC))))
  (if `Human?`
    (if (not (`local.bSpawnedFromSpawnTable`))
      (bind _layout (`self.GenerateHumanVisuals` HumanNPCType))
      (message `/Game/Characters/I_HasCharacterLayoutInterface.SetCharacterLayout` NPC _layout)
      (`self.SetItemsToEquip` HumanNPCType NPC))
    (elif (not (`KismetTextLibrary.EqualEqual_TextText` "" Name))
      (`ConanCharacter.SetCharacterName` NPC Name)))
  ;[1 1 1] Set Aggression from Behavior Parameters (humans only, as wildlife npcs have not gotten a pass yet)
  (bind _asbase_humanoid_npc (cast `/Game/Characters/NPCs/Humanoid/BaseHumanoidNPC` NPC)
    (:`then`
      (bind _asbp_human_default_behavior_paramters (cast `/Game/Systems/AI/BP_HumanDefaultBehaviorParamters` BehaviorParameters)
        (:`then`
          (set `/Game/Characters/BaseNPC.Aggression` (`/Game/Systems/AI/BP_HumanDefaultBehaviorParamters.Aggression` _asbp_human_default_behavior_paramters) _asbase_humanoid_npc))
        (:`CastFailed`
          _)))
    (:`CastFailed`
      _))
  (bind _ashuman_aicontroller (cast `/Game/Systems/AI/NewAI/HumanAIController` (`Pawn.GetController` NPC))
    (:`then`
      (`/Game/Systems/AI/NewAI/HumanAIController.SetBehaviorParameters` _ashuman_aicontroller BehaviorParameters)
      (return))
    (:`CastFailed`
      (return))))

(fn `FinishAsyncTrySpawnNPCFromSpawnTableLowLevel`
  (params (RowName :type Name) (SpawnLocation :type "Vector Structure") (RoamRadius_ :type "Float (double-precision)") (`StaticSpawnPoint_ (optional)` :type "StaticSpawnPoint Object Reference") (`TerritoryVolumeSpawner (optional)` :type "/Game/Systems/AI/BP_NPCTerritorySpawnerInterface Interface") (InputSpawnedNPC :type "Pawn Object Reference") (InputLayout :type "CharacterLayout Structure") (InputNPCBehaviorParameters :type "Object Class Reference") (SpawnerType :type "NpcSpawnerType Enum") (SpawnerIndex :type Integer))
  (returns (Success :type Boolean) (NPC :type "Pawn Object Reference") (CharacterLayout :type "CharacterLayout Structure"))
  (locals (Layout :type "CharacterLayout Structure") (NPCBehaviorParameters :type "Object Class Reference") (SpawnedNPC :type "Pawn Object Reference") (inSpawnLocation :type "Vector Structure") (RoamRadius :type "Float (double-precision)") (BehaviorClass :type "/Game/Systems/AI/BP_NPCBehaviorParameters Class Reference") (StaticSpawnPoint :type "StaticSpawnPoint Object Reference") (TerritoryVolumeSpawner :type "/Game/Systems/AI/BP_NPCTerritorySpawnerInterface Interface") (IsHuman :type Boolean) (SpawnerType_ :type "NpcSpawnerType Enum") (SpawnerIndex_ :type Integer))
  (bind _spawnerindex_ (`local.SpawnerIndex_`))
  (set `local.inSpawnLocation` SpawnLocation)
  (set `local.RoamRadius` RoamRadius_)
  (set `local.StaticSpawnPoint` `StaticSpawnPoint_ (optional)`)
  (set `local.TerritoryVolumeSpawner` `TerritoryVolumeSpawner (optional)`)
  (set `local.SpawnedNPC` InputSpawnedNPC)
  (set `local.Layout` InputLayout)
  (set `local.NPCBehaviorParameters` InputNPCBehaviorParameters)
  (set `local.SpawnerType_` SpawnerType)
  (set `local.SpawnerIndex_` SpawnerIndex)
  (bind _asbase_npc (cast `/Game/Characters/BaseNPC` (`local.SpawnedNPC`))
    (:`then`
      (bind _asbase_humanoid_npc (cast `/Game/Characters/NPCs/Humanoid/BaseHumanoidNPC` _asbase_npc)
        (:`then`
          (set `/Game/Characters/NPCs/Humanoid/BaseHumanoidNPC.CharacterLayout` (`local.Layout`) _asbase_humanoid_npc))
        (:`CastFailed`
          _))
      (bind (_npcstillalive _adjustedlocation) (`self.PlaceNPCOnGroundOrDie` (`local.inSpawnLocation`) false _asbase_npc))
      (if _npcstillalive
        (set `local.inSpawnLocation` _adjustedlocation)
        (bind _asbp_npcbehavior_parameters (castclass `/Game/Systems/AI/BP_NPCBehaviorParameters` (`local.NPCBehaviorParameters`))
          (:`then`
            (set `local.BehaviorClass` _asbp_npcbehavior_parameters))
          (:`CastFailed`
            (`/Game/Systems/BP_MacroGlobal.DebugPrintSimple` (`KismetStringLibrary.Concat_StrStr` "NPCTerritorySpawner::TrySpawnNPC called with invalid NPCBehaviorParamters for SpawnTableID: " (`KismetStringLibrary.Conv_NameToString` RowName)) "INFOL_DATAERROR" "SpawnTable"
              (:`Output`
                (set `local.BehaviorClass` "/Game/Systems/AI/BP_DefaultNPCBehaviorParameters.BP_DefaultNPCBehaviorParameters_C")))))
        (bind _returnvalue (`|GenericCreateObject` (`local.BehaviorClass`) _asbase_npc))
        (`self.ConfigureSpawnedNPC` "NewEnumerator3" (`local.IsHuman`) _asbase_npc _spawnerindex_ _spawnerindex_ _spawnerindex_ (`local.RoamRadius`) (`local.inSpawnLocation`) (`local.StaticSpawnPoint`) (`local.TerritoryVolumeSpawner`) _returnvalue true "" RowName)
        (bind _returnvalue_2 (`ConanCharacter.GetStatHolder` _asbase_npc))
        (`/Engine/EditorBlueprintResources/StandardMacros.IsValid` _returnvalue_2
          (:`Is Valid`
            (`StatHolder.SetIntStat` _returnvalue_2 "HealthCurrent" (`StatHolder.GetIntStat` _returnvalue_2 "HealthMax" "Full"))
            (`StatHolder.SetIntStat` _returnvalue_2 "StaminaCurrent" (`StatHolder.GetIntStat` _returnvalue_2 "StaminaMax" "Full"))
            (`StatHolder.SetIntStat` _returnvalue_2 "ConsciousnessCurrent" (`StatHolder.GetIntStat` _returnvalue_2 "ConsciousnessMax" "Full")))
          (:`Is Not Valid`
            _))
        (`/Game/Systems/BP_MacroGlobal.LogHeatmapEvent` "NewEnumerator3" "INFOL_INFO1" (`local.inSpawnLocation`) (`KismetSystemLibrary.GetDisplayName` _asbase_npc)
          (:`Output`
            (return true _asbase_npc (`local.Layout`))))
        (else
          (`LoggerLibrary.DWLogString` null "No Place found for the NPC" "Modding" "INFOL_CODEERROR")
          (return false null))))
    (:`CastFailed`
      (`LoggerLibrary.DWLogString` null "Failed to cast to BaseNPC" "Modding" "INFOL_CODEERROR")
      (return false null))))

(fn `GenerateHumanVisuals`
  (params (HumanType :type "/Game/Systems/Spawning/SpawnInputs/NPCHumans Enum"))
  (returns (Layout :type "CharacterLayout Structure"))
  (locals (TempLayout :type "CharacterLayout Structure"))
  (bind (_templayout_meshlayout _templayout_texturelayout _templayout_tintlayout _templayout_boolparams _templayout_intparams _templayout_scalarparams) (break `CharacterLayout` (`local.TempLayout`)))
  (bind _isfemale (break `CharacterBoolParameters` _templayout_boolparams))
  (`|ExecutionSequence`
    (:`then_0`
      (`CharacterFunctionLibrary.SetCharacterBoolSlot` _templayout_boolparams "IsFemale" (< (`KismetMathLibrary.RandomIntegerInRange` 1 4) 2)))
    (:`then_1`
      (`CharacterFunctionLibrary.SetCharacterMeshSlot` _templayout_meshlayout "Hair" (`KismetMathLibrary.RandomIntegerInRange` 0 (- (`/Game/Characters/CharacterAssembleLibrary.GetNumMeshesForCharacter` _isfemale "Hair") 1))))
    (:`then_2`
      (`CharacterFunctionLibrary.SetCharacterMeshSlot` _templayout_meshlayout "Head" (`KismetMathLibrary.RandomIntegerInRange` 0 (- (`/Game/Characters/CharacterAssembleLibrary.GetNumMeshesForCharacter` _isfemale "Head") 1))))
    (:`then_3`
      (bind _enumvalue (foreach `CharacterTintSlots`)
        (:`LoopBody`
          (`CharacterFunctionLibrary.SetCharacterTintSlot` _templayout_tintlayout _enumvalue (`KismetMathLibrary.RandomIntegerInRange` 0 (- (`/Game/Characters/CharacterAssembleLibrary.GetNumTintsForCharacter` _enumvalue) 1))))))
    (:`then_4`
      (bind _enumvalue_2 (foreach `CharacterTextureSlots`)
        (:`LoopBody`
          (`CharacterFunctionLibrary.SetCharacterTextureSlot` _templayout_texturelayout _enumvalue_2 (`KismetMathLibrary.RandomIntegerInRange` 0 (- (`/Game/Characters/CharacterAssembleLibrary.GetNumTexturesForCharacter` _isfemale _enumvalue_2) 1))))))
    (:`then_5`
      (`CharacterFunctionLibrary.SetCharacterScalarSlot` _templayout_scalarparams "Height" (`KismetMathLibrary.RandomFloatInRange` 0.9 1.1)))
    (:`then_6`
      (bind _returnvalue (`|GetDataTableRow` "/Game/Systems/Spawning/Humans/NPC_Human_Darfari_Cannibals_Items_DataTable.NPC_Human_Darfari_Cannibals_Items_DataTable" (`KismetStringLibrary.Conv_StringToName` (`KismetStringLibrary.Concat_StrStr` "Helmet_" (`|GetEnumeratorNameAsString` HumanType))))
        (:`then`
          (bind _vispieces (`self.CheckForInvalidDataTableValues` _returnvalue))
          (bind _randompiece (`self.RandomizedVisualPiece` _vispieces))
          (`CharacterFunctionLibrary.SetCharacterMeshSlot` _templayout_meshlayout "Helmet" _randompiece))))
    (:`then_7`
      (bind _returnvalue_2 (`|GetDataTableRow` "/Game/Systems/Spawning/Humans/NPC_Human_Darfari_Cannibals_Items_DataTable.NPC_Human_Darfari_Cannibals_Items_DataTable" (`KismetStringLibrary.Conv_StringToName` (`KismetStringLibrary.Concat_StrStr` "Hands_" (`|GetEnumeratorNameAsString` HumanType))))
        (:`then`
          (bind _vispieces_2 (`self.CheckForInvalidDataTableValues` _returnvalue_2))
          (bind _randompiece_2 (`self.RandomizedVisualPiece` _vispieces_2))
          (`CharacterFunctionLibrary.SetCharacterMeshSlot` _templayout_meshlayout "Hands" _randompiece_2))))
    (:`then_8`
      (bind _returnvalue_3 (`|GetDataTableRow` "/Game/Systems/Spawning/Humans/NPC_Human_Darfari_Cannibals_Items_DataTable.NPC_Human_Darfari_Cannibals_Items_DataTable" (`KismetStringLibrary.Conv_StringToName` (`KismetStringLibrary.Concat_StrStr` "UpperBody_" (`|GetEnumeratorNameAsString` HumanType))))
        (:`then`
          (bind _vispieces_3 (`self.CheckForInvalidDataTableValues` _returnvalue_3))
          (bind _randompiece_3 (`self.RandomizedVisualPiece` _vispieces_3))
          (`CharacterFunctionLibrary.SetCharacterMeshSlot` _templayout_meshlayout "Upperbody" _randompiece_3))))
    (:`then_9`
      (bind _returnvalue_4 (`|GetDataTableRow` "/Game/Systems/Spawning/Humans/NPC_Human_Darfari_Cannibals_Items_DataTable.NPC_Human_Darfari_Cannibals_Items_DataTable" (`KismetStringLibrary.Conv_StringToName` (`KismetStringLibrary.Concat_StrStr` "LowerBody_" (`|GetEnumeratorNameAsString` HumanType))))
        (:`then`
          (bind _vispieces_4 (`self.CheckForInvalidDataTableValues` _returnvalue_4))
          (bind _randompiece_4 (`self.RandomizedVisualPiece` _vispieces_4))
          (`CharacterFunctionLibrary.SetCharacterMeshSlot` _templayout_meshlayout "Lowerbody" _randompiece_4))))
    (:`then_10`
      (bind _returnvalue_5 (`|GetDataTableRow` "/Game/Systems/Spawning/Humans/NPC_Human_Darfari_Cannibals_Items_DataTable.NPC_Human_Darfari_Cannibals_Items_DataTable" (`KismetStringLibrary.Conv_StringToName` (`KismetStringLibrary.Concat_StrStr` "Feet_" (`|GetEnumeratorNameAsString` HumanType))))
        (:`then`
          (bind _vispieces_5 (`self.CheckForInvalidDataTableValues` _returnvalue_5))
          (bind _randompiece_5 (`self.RandomizedVisualPiece` _vispieces_5))
          (`CharacterFunctionLibrary.SetCharacterMeshSlot` _templayout_meshlayout "Feet" _randompiece_5))))
    (:`then_11`
      (return (`local.TempLayout`)))))

(fn `GetHomeLocationBBKey`
  (returns (HomeLocation :type Name))
  (return "HomeLocation"))

(fn `GetTerritorySpawnVolumeRadiusBBKey`
  (returns (TerritorySpawnVolumeRadius :type Name))
  (return "TerritorySpawnVolumeRadius"))

(fn `LogNPCSpawn`
  (params (SpawnLocation :type "Vector Structure") (NPC :type "Object Object Reference") (NPCRowIndex :type Integer) (NPCTypeName :type String))
  (`/Game/Systems/Interfaces/BaseGameModeInterface.NPCSpawned` (cast `/Game/Systems/Interfaces/BaseGameModeInterface` (`GameplayStatics.GetGameMode` null) :!pure true) NPCRowIndex NPCTypeName)
  (`/Game/Systems/BP_MacroGlobal.LogHeatmapEvent` "NewEnumerator3" "INFOL_INFO1" SpawnLocation (`KismetSystemLibrary.GetDisplayName` NPC)
    (:`Output`
      (return))))

(fn `PlaceNPCOnGroundOrDie`
  (params (SuggestedSpawnLocation :type "Vector Structure") (SpawnUnderneathRoof :type Boolean) (NPC :type "Character Object Reference"))
  (returns (NPCStillAlive :type Boolean) (AdjustedLocation :type "Vector Structure"))
  (locals (HasLocation :type Boolean) (BestLocation :type "Vector Structure") (SuggestedLocation :type "Vector Structure"))
  (bind _suggestedlocation (`local.SuggestedLocation`))
  (bind (_suggestedlocation_x _suggestedlocation_y _suggestedlocation_z) (`KismetMathLibrary.BreakVector` (`local.SuggestedLocation`)))
  (bind (_bestlocation_x _bestlocation_y _bestlocation_z) (`KismetMathLibrary.BreakVector` (`local.BestLocation`)))
  (bind _capsulecomponent (`Character.CapsuleComponent` NPC))
  (if (not (< SuggestedSpawnLocation_Z 0.0))
    (set `local.SuggestedLocation` (`KismetMathLibrary.MakeVector` SuggestedSpawnLocation_X SuggestedSpawnLocation_Y (+ SuggestedSpawnLocation_Z 1000.0)))
    (else
      (set `local.SuggestedLocation` (`KismetMathLibrary.MakeVector` SuggestedSpawnLocation_X SuggestedSpawnLocation_Y (- SuggestedSpawnLocation_Z 1000.0)))))
  (`LoggerLibrary.DWLogString` null (`KismetStringLibrary.BuildString_Vector` "" "Suggested Location [" (`local.SuggestedLocation`) "]") "Modding" "INFOL_IMPORTANT")
  (bind _outhits (`KismetSystemLibrary.CapsuleTraceMultiForObjects` null (+ _suggestedlocation (`KismetMathLibrary.MakeVector` 0.0 0.0 (`KismetMathLibrary.SelectFloat` 0.0 500000.0 SpawnUnderneathRoof))) (- _suggestedlocation (`KismetMathLibrary.MakeVector` 0.0 0.0 500000.0)) (`CapsuleComponent.GetScaledCapsuleRadius` _capsulecomponent) (`CapsuleComponent.GetScaledCapsuleHalfHeight` _capsulecomponent) (`|MakeArray` "ObjectTypeQuery1" "ObjectTypeQuery2" "ObjectTypeQuery13" "ObjectTypeQuery10" :!type "EObjectTypeQuery Enum") false (`|MakeArray` NPC :!type "Actor Object Reference")))
  (set `local.HasLocation` false)
  (for _array_element _outhits
    ;[1 1 1] Pick closest blocking hit with upwards-pointing impact normal.
    (`/Engine/EditorBlueprintResources/StandardMacros.IsValid` (`.HitComponent` (`GameplayStatics.BreakHitResult` _array_element))
      (:`Is Valid`
        (if (and (`|EnumEquality` (`PrimitiveComponent.GetCollisionResponseToChannel` (`.HitComponent` (`GameplayStatics.BreakHitResult` _array_element)) "ECC_Pawn") "ECR_Block") (> (.z (`.ImpactNormal` (`GameplayStatics.BreakHitResult` _array_element))) 0.0))
          (if (`local.HasLocation`)
            (if (< (`KismetMathLibrary.Abs` (- (.z (`.Location` (`GameplayStatics.BreakHitResult` _array_element))) _suggestedlocation_z)) (`KismetMathLibrary.Abs` (- _suggestedlocation_z _bestlocation_z)))
              (set `local.BestLocation` (`.Location` (`GameplayStatics.BreakHitResult` _array_element)) :!label _label))
            (else
              (set `local.HasLocation` true)
              (goto _label)))))))
  (if (`local.HasLocation`)
    (`Actor.K2_SetActorLocation` NPC (`local.BestLocation`) false true)
    (return true (`local.BestLocation`))
    (else
      (`Actor.K2_DestroyActor` NPC)
      (return false (0.0 0.0 0.0)))))

(fn `RandomizedVisualPiece`
  (params (VisPieces :type "Array of Integer"))
  (returns (RandomPiece :type Integer))
  (bind _returnvalue (`KismetArrayLibrary.Array_Length` VisPieces))
  (if (> _returnvalue 0)
    (return (`KismetArrayLibrary.Array_Get` VisPieces (`KismetMathLibrary.RandomIntegerInRange` 0 (- _returnvalue 1))))
    (else
      (return -1))))

(fn `SetItemsToEquip`
  (params (NPCType :type "/Game/Systems/Spawning/SpawnInputs/NPCHumans Enum") (NPC :type "/Game/Characters/BaseNPC Object Reference"))
  (bind _returnvalue (`|GetEnumeratorNameAsString` NPCType))
  (bind _returnvalue_2 (`KismetStringLibrary.Concat_StrStr` "MainHand_" _returnvalue))
  (bind _returnvalue_3 (`KismetStringLibrary.Concat_StrStr` "OffHand_" _returnvalue))
  (`/Game/Systems/BP_MacroGlobal.DebugPrintSimple` (`KismetStringLibrary.Concat_StrStr` "Looking up " _returnvalue_2 " and " _returnvalue_3 "...") "INFOL_INFO0" "AI"
    (:`Output`
      (bind _returnvalue_4 (`|GetDataTableRow` "/Game/Systems/Spawning/Humans/NPC_Human_Items_DataTable.NPC_Human_Items_DataTable" (`KismetStringLibrary.Conv_StringToName` _returnvalue_2))
        (:`then`
          (bind _vispieces (`self.CheckForInvalidDataTableValues` _returnvalue_4))
          (bind _randompiece (`self.RandomizedVisualPiece` _vispieces))
          (set `/Game/Characters/BaseNPC.NPCDefaultMainHand` _randompiece NPC)
          (bind _returnvalue_5 (`|GetDataTableRow` "/Game/Items/ItemTable.ItemTable" (`KismetStringLibrary.Conv_StringToName` (`KismetStringLibrary.Conv_IntToString` _randompiece)))
            (:`then`
              (if (not (`|EnumEquality` (`.WeaponArcheType` (break `ItemTableRow` _returnvalue_5)) "TwoHanded"))
                (bind _returnvalue_6 (`|GetDataTableRow` "/Game/Systems/Spawning/Humans/NPC_Human_Items_DataTable.NPC_Human_Items_DataTable" (`KismetStringLibrary.Conv_StringToName` _returnvalue_3))
                  (:`then`
                    (bind _vispieces_2 (`self.CheckForInvalidDataTableValues` _returnvalue_6))
                    (bind _randompiece_2 (`self.RandomizedVisualPiece` _vispieces_2))
                    (set `/Game/Characters/BaseNPC.NPCDefaultOffHand` _randompiece_2 NPC)
                    (`|GetDataTableRow` "/Game/Items/ItemTable.ItemTable" (`KismetStringLibrary.Conv_StringToName` (`KismetStringLibrary.Conv_IntToString` _randompiece_2)))))))))))))

(fn `TrySpawnNPCLowLevel`
  (params (BehaviorTree :type "BehaviorTree Object Reference") (`Rotation Z (Yaw)` :type "Float (double-precision)") (PawnClass :type "Pawn Class Reference") (ControllerClass :type "AIController Class Reference") (SuggestedSpawnLocation :type "Vector Structure") (RoamRadius_ :type "Float (double-precision)") (MessagePrefix :type String) (`NPCRowIndex (optional)` :type Integer) (`NPCTypeName (optional)` :type String) (SpawnUnderneathRoof_ :type Boolean) (`HumanNPCType (humans only)` :type "/Game/Systems/Spawning/SpawnInputs/NPCHumans Enum") (`Human?_` :type Boolean) (`SpawnerHumanNPCIndex (with spawner only)` :type Integer) (`SpawnerWildlifeNPCIndex (with spawner only)` :type Integer) (`SpawnerSpawnPointIndex (with spawner only)` :type Integer) (`TerritoryVolumeSpawner (optional)` :type "/Game/Systems/AI/BP_NPCTerritorySpawnerInterface Interface") (`StaticSpawnPoint_ (optional)` :type "StaticSpawnPoint Object Reference") (`BehaviorParameters (optional)` :type "/Game/Systems/AI/BP_NPCBehaviorParameters Object Reference") (Name :type Text) (RowName :type Name))
  (returns (Success :type Boolean) (NPC :type "ConanCharacter Object Reference"))
  (locals (MessagePrefix_ :type String) (SpawnUnderneathRoof :type Boolean) (NPCRowIndex_ :type Integer) (NPCTypeName_ :type String) (SpawnerHumanNPCIndex_ :type Integer) (SpawnerWildlifeNPCIndex_ :type Integer) (RoamRadius :type "Float (double-precision)") (TerritoryVolumeSpawner :type "/Game/Systems/AI/BP_NPCTerritorySpawnerInterface Interface") (StaticSpawnPoint :type "StaticSpawnPoint Object Reference") (HumanNPCType_ :type "/Game/Systems/Spawning/SpawnInputs/NPCHumans Enum") (HumanNPCTribe_ :type "/Game/Systems/Spawning/SpawnInputs/NPCHumansTribeList Enum") (`Human?` :type Boolean) (BehaviorParameters_ :type "/Game/Systems/AI/BP_NPCBehaviorParameters Object Reference") (ControllerClass_ :type "AIController Class Reference") (`Local Name` :type Text) (SpawnerStaticSpawnpointIndex_ :type Integer) (LocalRowName :type Name))
  (`|ExecutionSequence`
    (:`then_0`
      (set `local.ControllerClass_` ControllerClass))
    (:`then_1`
      (set `local.RoamRadius` RoamRadius_))
    (:`then_2`
      (set `local.MessagePrefix_` MessagePrefix))
    (:`then_3`
      (set `local.NPCRowIndex_` `NPCRowIndex (optional)`))
    (:`then_4`
      (set `local.NPCTypeName_` `NPCTypeName (optional)`))
    (:`then_5`
      (set `local.SpawnUnderneathRoof` SpawnUnderneathRoof_))
    (:`then_6`
      (set `local.HumanNPCType_` `HumanNPCType (humans only)`))
    (:`then_7`
      (set `local.Human?` `Human?_`))
    (:`then_8`
      (set `local.SpawnerHumanNPCIndex_` `SpawnerHumanNPCIndex (with spawner only)`))
    (:`then_9`
      (set `local.SpawnerWildlifeNPCIndex_` `SpawnerWildlifeNPCIndex (with spawner only)`))
    (:`then_10`
      (set `local.SpawnerStaticSpawnpointIndex_` `SpawnerSpawnPointIndex (with spawner only)`))
    (:`then_11`
      (set `local.TerritoryVolumeSpawner` `TerritoryVolumeSpawner (optional)`))
    (:`then_12`
      (set `local.StaticSpawnPoint` `StaticSpawnPoint_ (optional)`))
    (:`then_13`
      (set `local.BehaviorParameters_` `BehaviorParameters (optional)`))
    (:`then_14`
      (set `local.Local Name` Name))
    (:`then_15`
      (set `local.LocalRowName` RowName))
    (:`then_16`
      (bind _returnvalue (`AIBlueprintHelperLibrary.SpawnAIFromClass` null PawnClass (`local.ControllerClass_`) BehaviorTree SuggestedSpawnLocation (`KismetMathLibrary.MakeRotator` 0.0 0.0 `Rotation Z (Yaw)`) true))
      (bind _asbase_npc (cast `/Game/Characters/BaseNPC` _returnvalue)
        (:`then`
          (bind (_npcstillalive _adjustedlocation) (`self.PlaceNPCOnGroundOrDie` SuggestedSpawnLocation (`local.SpawnUnderneathRoof`) _asbase_npc))
          (if _npcstillalive
            (`self.ConfigureSpawnedNPC` (`local.HumanNPCType_`) (`local.Human?`) _asbase_npc (`local.SpawnerHumanNPCIndex_`) (`local.SpawnerWildlifeNPCIndex_`) (`local.SpawnerStaticSpawnpointIndex_`) (`local.RoamRadius`) _adjustedlocation (`local.StaticSpawnPoint`) (`local.TerritoryVolumeSpawner`) (`local.BehaviorParameters_`) false (`local.Local Name`) (`local.LocalRowName`))
            (`self.LogNPCSpawn` _adjustedlocation _asbase_npc (`local.NPCRowIndex_`) (`local.NPCTypeName_`))
            (return true _asbase_npc)
            (else
              (`/Game/Systems/BP_MacroGlobal.LogHeatmapEvent` "NewEnumerator4" "INFOL_CODEWARNING" _adjustedlocation (`KismetSystemLibrary.GetDisplayName` _asbase_npc)
                (:`Output`
                  (`LoggerLibrary.DWLogString` null (`KismetStringLibrary.Concat_StrStr` (`local.MessagePrefix_`) "Capsule trace failed. There is no ground to spawn the NPC on.") "AI" (select `bool` (`KismetSystemLibrary.IsDedicatedServer` null) :`false` "INFOL_INFO0" :`true` "INFOL_DATAWARNING" :!type "EDebugLevel Enum")))))))
        (:`CastFailed`
          (`/Game/Systems/BP_MacroGlobal.LogHeatmapEvent` "NewEnumerator4" "INFOL_CODEWARNING" SuggestedSpawnLocation (`KismetSystemLibrary.GetClassDisplayName` PawnClass)
            (:`Output`
              (`LoggerLibrary.DWLogString` null (`KismetStringLibrary.Concat_StrStr` (`local.MessagePrefix_`) "Spawn call failed. Failed cast to BaseNPC. Pawn: " (`KismetSystemLibrary.GetClassDisplayName` PawnClass) ". Behavior Tree: " (`KismetSystemLibrary.GetDisplayName` BehaviorTree) "This is likely because it is attempting to spawn inside something.") "AI" "INFOL_CODEWARNING")))))
      (return false null))))