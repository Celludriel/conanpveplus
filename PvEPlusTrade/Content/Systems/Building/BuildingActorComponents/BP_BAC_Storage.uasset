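; Building actor component that makes placed storage containers such as chests interactable, opening the crafting GUI for the player.
; Interaction toggles a list of current users, with first-in and last-out driving multicast open/close animation and sound; deselection also removes users.
; An optional key item gates access and is consumed when the pawn has a BP_LoreInteractor.
; BeginPlay caches the animation instance and loads persisted inventory; closing saves the actor.
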(event `OpenGui`
  (params (Instigator :type "PlayerController Object Reference"))
  ;[1 1 1] Handle GUI
  (`ConanCharacter.SetInteractingActor` (cast `ConanCharacter` (`Controller.K2_GetPawn` Instigator) :!pure true) (`self.GetOwner`) "CraftingGUI"))

(event `CloseGui`
  (params (Instigator :type "PlayerController Object Reference"))
  ;[1 1 1] Handle GUI
  (`ConanCharacter.SetInteractingActor` (cast `ConanCharacter` (`Controller.K2_GetPawn` Instigator) :!pure true) null "None"))

(event `CheckStateAndClose`
  (params (Instigator :type "PlayerController Object Reference"))
  (if (`KismetArrayLibrary.Array_Contains` (`self.PlayersInteractingWithChest`) Instigator)
    (`KismetArrayLibrary.Array_RemoveItem` (`self.PlayersInteractingWithChest`) Instigator)
    (if (== (`KismetArrayLibrary.Array_Length` (`self.PlayersInteractingWithChest`)) 0)
      (`self.CloseChest`))))

(event `CheckState`
  (params (Instigator :type "PlayerController Object Reference"))
  (bind _playersinteractingwithchest (`self.PlayersInteractingWithChest`))
  (if (`KismetArrayLibrary.Array_Contains` (`self.PlayersInteractingWithChest`) Instigator)
    (`KismetArrayLibrary.Array_RemoveItem` (`self.PlayersInteractingWithChest`) Instigator)
    (`self.CloseGui` Instigator)
    (if (== (`KismetArrayLibrary.Array_Length` (`self.PlayersInteractingWithChest`)) 0)
      (`self.CloseChest`))
    (else
      (if (== (`KismetArrayLibrary.Array_Length` (`self.PlayersInteractingWithChest`)) 0)
        (`KismetArrayLibrary.Array_Add` _playersinteractingwithchest Instigator)
        (`self.OpenChest`)
        (else
          (`KismetArrayLibrary.Array_Add` _playersinteractingwithchest Instigator)))
      (`self.OpenGui` Instigator))))

(event `InteractableInterface.InteractableActivate`
  (params (Component :type "PrimitiveComponent Object Reference") (Instigator :type "PlayerController Object Reference") (HitIndex :type Integer))
  (bind _returnvalue (`Controller.K2_GetPawn` Instigator))
  (bind _asconan_character (cast `ConanCharacter` _returnvalue :!pure true))
  (if (`self.RequiresKey`)
    (if (`ItemInventory.HasItemByTemplateID` (`ItemInventory.GetInventoryByType` _returnvalue "Backpack") (`self.ItemIDRequired`) 1)
      (`self.CheckState` Instigator)
      (if (> (`KismetArrayLibrary.Array_Length` (`Actor.K2_GetComponentsByClass` _returnvalue "/Game/Items/LoreObjects/BP_LoreInteractor.BP_LoreInteractor_C")) 0)
        (bind _returnvalue_2 (`ConanCharacter.GetBackpackInventory` _asconan_character))
        (`ItemInventory.DeleteItemsByTemplate` _returnvalue_2 (`self.ItemIDRequired`) 1))
      (else
        (`ConanCharacter.ClientHUDShowNotification` _asconan_character (`self.NeedKeyText`) false)))
    (else
      (`self.CheckState` Instigator))))

(event `InteractableInterface.InteractableSelectionChanged`
  (params (IsSelected :type Boolean) (Instigator :type "PlayerController Object Reference") (InstanceIndex :type Integer))
  (if (not IsSelected)
    (`self.CheckStateAndCLose` Instigator)))

(event `OpenChest`
  (`self.Multicast_OpenChest`))

(event `Multicast_OpenChest`
  (bind _sound_open (`self.Sound_Open`))
  (bind _animinstance (`self.AnimInstance`))
  (`/Engine/EditorBlueprintResources/StandardMacros.IsValid` _animinstance
    (:`Is Valid`
      (message `/Game/Master_AnimBP/BP_HasBinaryStatesInterface.SetOpen` _animinstance))
    (:`Is Not Valid`
      _))
  (set `self.OpenState` true)
  (`/Engine/EditorBlueprintResources/StandardMacros.IsValid` _sound_open
    (:`Is Valid`
      (`GameplayStatics.PlaySoundAtLocation` _sound_open (`Actor.K2_GetActorLocation` (`self.GetOwner`))))))

(event `CloseChest`
  (`self.Multicast_CloseChest`)
  (`WorldPersistenceComponent.SaveActor` (`self.GetOwner`)))

(event `Multicast_CloseChest`
  (bind _animinstance (`self.AnimInstance`))
  (bind _sound_close (`self.Sound_Close`))
  (`/Engine/EditorBlueprintResources/StandardMacros.IsValid` _animinstance
    (:`Is Valid`
      (message `/Game/Master_AnimBP/BP_HasBinaryStatesInterface.SetClosed` _animinstance))
    (:`Is Not Valid`
      _))
  (set `self.OpenState` false)
  (`/Engine/EditorBlueprintResources/StandardMacros.IsValid` _sound_close
    (:`Is Valid`
      (`GameplayStatics.PlaySoundAtLocation` _sound_close (`Actor.K2_GetActorLocation` (`self.GetOwner`))))))

(event `self.ReceiveBeginPlay`
  (bind _returnvalue (`self.GetOwner`))
  ;[1 1 1] Begin play
  (`|ExecutionSequence`
    (:`then_0`
      (for _array_element (`Actor.K2_GetComponentsByClass` (`self.GetOwner`) "/Script/Engine.SkeletalMeshComponent")
        (set `self.AnimInstance` (`SkeletalMeshComponent.GetAnimInstance` _array_element))))
    (:`then_1`
      (for _array_element_2 (`Actor.K2_GetComponentsByClass` _returnvalue "/Script/ConanSandbox.ConanBuildingPersistenceComponent")
        (bind (_uid _result) (`LoadInventoryCallProxy.LoadInventory` (`PersistenceComponent.GetUniqueID` _array_element_2))
          (:`OnSuccess`
            (`LoadInventoryCallProxy.ProcessInventoryData` _returnvalue _result)))))))